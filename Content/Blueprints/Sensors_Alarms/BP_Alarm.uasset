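; BP_Alarm is an alarm actor for a stealth game that raises a facility-wide alert.
; StartAlarm plays a sound at its location, unhides two spotlights and calls AlertAllGuards, guarded by an active flag.
; AlertAllGuards sets HasSeenPlayer on every guard's AI blackboard and has GM_Stealth switch to escape music.
; StopAlarm hides the lights and fades out the sound, leaving guard and music state untouched.
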(event Custom|Start%20Alarm
  (if (not (Variables|Default|GetAlarm%20Active))
    (bind _returnvalue (Audio|SpawnSoundatLocation "/Game/Audio/Alarms/MS_Alarm.MS_Alarm" (Transformation|GetActorLocation) "0, 0, 0" 1.0 1.0 0.0 0 0))
    (Variables|Default|SetAlarm%20sound _returnvalue)
    (Variables|Default|SetAlarm%20Active true)
    (Development|SetHiddeninGame (Variables|Default|GetSpotLight1) false false)
    (CallFunction|AlertAllGuards)))

(event Custom|Stop%20Alarm
  (if (Variables|Default|GetAlarm%20Active)
    (Development|SetHiddeninGame (Variables|Default|GetSpotLight1) true false)
    (Audio|Components|Audio|FadeOut (Variables|Default|GetAlarm%20sound) 0.5 0.0 "Linear" :!class /Script/Engine.AudioComponent)
    (Variables|Default|SetAlarm%20Active false)))

(event Custom|Alert%20All%20Guards
  (bind _outactors (Actor|GetAllActorsOfClass "/Game/IA/BP_Guard.BP_Guard_C"))
  (for _array_element _outactors
    (bind _asbp_ia_guard (Utilities|Casting|CastToBP_IA_Guard (AI|GetAIController _array_element)))
    (AI|Components|Blackboard|SetValueasBool (AI|GetBlackboard _asbp_ia_guard) (Utilities|Name|MakeLiteralName "HasSeenPlayer") true))
  (bind _asgm_stealth (Utilities|Casting|CastToGM_Stealth (Game|GetGameMode)))
  (Default|SwitchMusictoScaping _asgm_stealth))

(fn ConstructionScript)