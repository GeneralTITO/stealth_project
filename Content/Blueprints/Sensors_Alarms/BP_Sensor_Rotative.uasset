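; Rotating alarm sensor that detects the player inside its trigger zone.
; The Motion timeline swings the Head back and forth across a 180-degree arc, with a FlipFlop alternating reverse and replay.
; A Player-tagged overlap starts a fast looping timer that accumulates TimeUnderZone, calls UpdateProgressBar (empty here) and calls DetectPlayer once the threshold is reached.
; The file has no end-overlap handling to stop or reset the count.
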(event OnComponentBeginOverlap(TriggerDetectionZone)
  (params (OverlappedComponent :type Primitive%20Component%20Object%20Reference) (OtherActor :type Actor%20Object%20Reference) (OtherComp :type Primitive%20Component%20Object%20Reference) (OtherBodyIndex :type Integer) (bFromSweep :type Boolean) (SweepResult :type Hit%20Result%20Structure%20%28by%20ref%29))
  (if (Actor|ActorHasTag OtherActor "Player")
    (Variables|Default|SetPlayer%20in%20zone true)
    (bind _returnvalue (Utilities|Time|SetTimerbyEvent (delegate Custom|Count) 0.002 true))
    (Variables|Default|SetCount%20timer _returnvalue)))

(event Custom|Count
  (Variables|Default|SetTime%20under%20zone (+ (Variables|Default|GetTime%20under%20zone) 0.005))
  (CallFunction|UpdateProgressBar)
  (if (>= (Variables|Default|GetTime%20under%20zone) 3.0)
    (CallFunction|DetectPlayer (stale OnComponentBeginOverlap(TriggerDetectionZone) OtherActor))))

(event Custom|Update%20Progress%20Bar)

(event EventBeginPlay
  (bind _rotation (Timeline|motion Play)
    (:Update
      (Transformation|SetRelativeRotation (Variables|Default|Gethead) (Math|Rotator|Lerp(Rotator) "0.000000,90.000000,0.000000" "0.000000,-90.000000,0.000000" _rotation) false false))
    (:Finished
      (Utilities|FlowControl|FlipFlop
        (:A
          (Timeline|motion Reverse))
        (:B
          (Timeline|motion PlayFromStart))))))

(fn ConstructionScript
  (|CallParentFunction))