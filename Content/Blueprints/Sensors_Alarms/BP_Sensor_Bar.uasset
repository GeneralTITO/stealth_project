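; Toggleable bar sensor from the alarm set that detects the player crossing its collision box.
; Box overlap passes the other actor to DetectPlayer, whose logic is not in this graph.
; Interact flips IsActiveSensor, switching actor collision and the visibility of ten bar components together.
; Each toggle also prints a colored Portuguese on-screen debug message for the activated or deactivated state.
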(event OnComponentBeginOverlap(boxcolision)
  (params (OverlappedComponent :type Primitive%20Component%20Object%20Reference) (OtherActor :type Actor%20Object%20Reference) (OtherComp :type Primitive%20Component%20Object%20Reference) (OtherBodyIndex :type Integer) (bFromSweep :type Boolean) (SweepResult :type Hit%20Result%20Structure%20%28by%20ref%29))
  (CallFunction|DetectPlayer OtherActor))

(event EventBeginPlay)

(event Collision|EventActorBeginOverlap
  (params (OtherActor :type Actor%20Object%20Reference)))

(event EventTick
  (params (DeltaSeconds :type Float%20%28single-precision%29)))

(event EventInteract
  (if (not (Variables|Default|GetIsActiveSensor))
    (Collision|SetActorEnableCollision true)
    (Development|PrintString "ativado" true true "(R=0.000000,G=1.000000,B=0.069329,A=1.000000)" 1e+01)
    (Rendering|SetVisibility (Variables|Default|GetBar%205) true false)
    (Variables|Default|SetIsActiveSensor true)
    (else
      (Collision|SetActorEnableCollision false)
      (Development|PrintString "desativado" true true "(R=1.000000,G=0.019096,B=0.000000,A=1.000000)" 1e+01)
      (Rendering|SetVisibility (Variables|Default|GetBar%205) false false)
      (Variables|Default|SetIsActiveSensor false))))

(fn ConstructionScript
  (|CallParentFunction))