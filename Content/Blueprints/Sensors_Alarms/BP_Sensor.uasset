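; Sensor Blueprint that triggers the level's alarm when it detects the player.
; DetectPlayer accepts only actors tagged Player and latches HasDetected, so it fires only once.
; On detection it calls StartAlarm on the BP_Alarm found by class lookup, then plays a Timeline that drives its point light's intensity.
; The file defines no caller for DetectPlayer, and the construction script is empty.
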(event Custom|Detect%20Player
  (params (Actor%20Detected :type Actor%20Object%20Reference))
  (if (and (Actor|ActorHasTag Actor%20Detected "Player") (not (Variables|Default|GetHasDetected)))
    (Variables|Default|SetHasDetected true)
    (bind _returnvalue (Actor|GetActorOfClass "/Game/Blueprints/Sensors_Alarms/BP_Alarm.BP_Alarm_C"))
    (Default|StartAlarm _returnvalue false)
    (bind _intensity_light (Timeline|Timeline Play)
      (:Update
        (Rendering|Components|Light|SetIntensity (Variables|Default|GetPointLight) (Math|Float|Lerp 0.0 1e+05 _intensity_light))))))

(fn ConstructionScript)