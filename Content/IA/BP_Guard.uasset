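; BP_Guard is a stealth enemy guard that can catch the player or be taken down.
; Catch plays a montage whose notify sphere-traces ahead and calls Captured once on GM_Stealth if it hits the player.
; Takedown, gated by CanTakedown, plays a victim montage, returns a reference pose for alignment and triggers a delayed ragdoll death.
; An overlap radius toggles the takedown prompt, and Run raises walk speed.
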(event OnComponentBeginOverlap(takedownradius)
  (params (OverlappedComponent :type Primitive%20Component%20Object%20Reference) (OtherActor :type Actor%20Object%20Reference) (OtherComp :type Primitive%20Component%20Object%20Reference) (OtherBodyIndex :type Integer) (bFromSweep :type Boolean) (SweepResult :type Hit%20Result%20Structure%20%28by%20ref%29))
  (if (and (Actor|ActorHasTag OtherActor "Player") (not (Variables|Default|GetIsDead)))
    (Rendering|SetVisibility (Variables|Default|GetTakedown%20Prompt%20Widget) true false)))

(event OnComponentEndOverlap(takedownradius)
  (params (OverlappedComponent :type Primitive%20Component%20Object%20Reference) (OtherActor :type Actor%20Object%20Reference) (OtherComp :type Primitive%20Component%20Object%20Reference) (OtherBodyIndex :type Integer))
  (if (Actor|ActorHasTag OtherActor "Player")
    (Rendering|SetVisibility (Variables|Default|GetTakedown%20Prompt%20Widget) false false)))

(event Custom|Takedown%20Ragdoll
  (Utilities|FlowControl|Delay 1.3)
  (Collision|SetCollisionEnabled (Variables|Character|GetMesh) "QueryAndPhysics")
  (Physics|SetSimulatePhysics (Variables|Character|GetMesh) true)
  (Pawn|Components|CharacterMovement|SetMovementMode (Variables|Character|GetCharacterMovement) "MOVE_None" 0)
  (Variables|Default|SetIsDead true))

(event EventRun
  (Variables|/Script/Engine.CharacterMovementComponent|SetMaxWalkSpeed (Variables|Character|GetCharacterMovement) 6e+02))

(event EventCatch
  (bind _returnvalue (Transformation|GetActorLocation))
  (if (not (Variables|Default|GetisAttacking))
    (Animation|Montage|PlayMontage (Variables|Character|GetMesh) "/Game/Characters/Player/Catch/Catch_Montage.Catch_Montage"
      (:then
        (Variables|Default|SetisAttacking true))
      (:OnCompleted
        (Variables|Default|SetisAttacking false))
      (:OnNotifyBegin
        (bind (_outhit _returnvalue_2) (Collision|SphereTraceForObjects _returnvalue (+ _returnvalue (* (Transformation|GetActorForwardVector) 135.0)) 1.2e+02 (Utilities|Array|MakeArray "ObjectTypeQuery3") false 0 "ForDuration"))
        (if _returnvalue_2
          (if (Actor|ActorHasTag (.HitActor (Collision|BreakHitResult _outhit)) "Player")
            (Utilities|FlowControl|DoOnce false
              (:Completed
                (bind _asgm_stealth (Utilities|Casting|CastToGM_Stealth (Game|GetGameMode)))
                (Default|Captured _asgm_stealth)))))))))

(fn ConstructionScript)

(fn Takedown
  (if (Variables|Default|GetCan%20Takedown)
    (Animation|PlayAnimMontage "/Game/Characters/Player/Takedowns/Takedown_Victim_Montage.Takedown_Victim_Montage" 1.0 "None")
    (CallFunction|TakedownRagdoll)
    (return (Transformation|GetWorldLocation (Variables|Default|GetREF)) (Transformation|GetActorRotation) (Variables|Default|GetCan%20Takedown) (Components|GetOwner (Variables|Character|GetMesh)))))